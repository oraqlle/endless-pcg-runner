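; BP_TileGen_01a is a tile generator actor that spawns BP_Tile_01a tiles in a chain.
; On BeginPlay it seeds the spawn point from its root transform and spawns the initial tile.
; AddTile spawns at the stored point, then advances that point to the new tile's attach point transform.
; Each tile receives references to the generator and previous tile, plus an initial-tile flag.
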(event EventBeginPlay
  (Variables|Default|SetNextTileSpawnPoint (Transformation|GetWorldTransform (Variables|Default|GetDefaultSceneRoot self)))
  (CallFunction|AddTile 0 true))

(event Collision|EventActorBeginOverlap
  (params (OtherActor :type Actor%20Object%20Reference)))

(event EventTick
  (params (DeltaSeconds :type Float%20%28single-precision%29)))

(fn ConstructionScript)

(fn AddTile
  (params (PrevTile :type BP%20Tile%2001a%20Object%20Reference) (InitialTile :type Boolean))
  (bind _returnvalue (Game|SpawnActorfromClass "/Game/Blueprints/BP_Tile_01a.BP_Tile_01a_C" (Variables|Default|GetNextTileSpawnPoint) "Undefined" "MultiplyWithRoot" 0 0))
  (bind _attachpointtransform (Default|GetAttachPointTransform _returnvalue))
  (Variables|Default|SetNextTileSpawnPoint _attachpointtransform)
  (Variables|/Game/Blueprints/BP_Tile_01a.BP_Tile_01a_C|SetGenSource _returnvalue self)
  (Variables|/Game/Blueprints/BP_Tile_01a.BP_Tile_01a_C|SetPrevTile _returnvalue PrevTile)
  (Variables|/Game/Blueprints/BP_Tile_01a.BP_Tile_01a_C|SetInitialTile _returnvalue InitialTile))