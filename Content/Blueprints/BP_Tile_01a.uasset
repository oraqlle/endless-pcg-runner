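; BP_Tile_01a is a tile that chains onto others through a generator as the first-person character advances.
; Overlapping its LoadTrigger with that character asks GenSource once to add the next tile, passing itself as the previous one.
; Non-initial tiles then destroy their predecessor after the generator's delay, so old tiles are cleaned up behind the player.
; GetAttachPointTransform exposes the AttachPoint's world transform.
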(event OnComponentBeginOverlap(LoadTrigger)
  (params (OverlappedComponent :type Primitive%20Component%20Object%20Reference) (OtherActor :type Actor%20Object%20Reference) (OtherComp :type Primitive%20Component%20Object%20Reference) (OtherBodyIndex :type Integer) (bFromSweep :type Boolean) (SweepResult :type Hit%20Result%20Structure%20%28by%20ref%29))
  (bind _gensource (Variables|Default|GetGenSource))
  (if (not (Variables|Default|GetNextTileLoaded))
    (Utilities|Casting|CastToBP_FirstPersonCharacter OtherActor)
    (Default|AddTile _gensource self false)
    (Variables|Default|SetNextTileLoaded true)
    (if (Math|Boolean|NORBoolean (Variables|Default|GetPrevTileDestroyed) (Variables|Default|GetInitialTile))
      (Utilities|FlowControl|Delay (Variables|/Game/Blueprints/BP_TileGen_01a.BP_TileGen_01a_C|GetTileDestroyDelay _gensource))
      (Actor|DestroyActor (Variables|Default|GetPrevTile))
      (Variables|Default|SetPrevTileDestroyed true))))

(event EventBeginPlay)

(event Collision|EventActorBeginOverlap
  (params (OtherActor :type Actor%20Object%20Reference)))

(event EventTick
  (params (DeltaSeconds :type Float%20%28single-precision%29)))

(fn ConstructionScript)

(fn GetAttachPointTransform
  (return (Transformation|GetWorldTransform (Variables|Default|GetAttachPoint))))